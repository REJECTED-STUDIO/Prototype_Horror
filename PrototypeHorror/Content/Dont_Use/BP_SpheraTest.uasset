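; Test sphere Blueprint that changes its collision and appearance when the active character switches between Lucia and Nyxa.
; The CharacterSwitch event passes the character to SetCollision and SetMaterial, which each branch on it.
; For Lucia the sphere blocks all channels and shows the arrow material; for Nyxa it ignores all channels and shows the disc material.
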(event `/Game/Blueprints/SwitchCharacter/BPI_SwitchCharacter.CharacterSwitch`
  (params (Characters :type "/Game/Blueprints/SwitchCharacter/E_Character Enum" :default "NewEnumerator0"))
  (`self.Set Collision` Characters)
  (`self.Set Material` Characters))

(fn `Set Collision`
  (params (NewParam :type "/Game/Blueprints/SwitchCharacter/E_Character Enum" :default "NewEnumerator0"))
  (bind _sphere (`self.Sphere`))
  (switch `/Game/Blueprints/SwitchCharacter/E_Character` NewParam
    (:`NewEnumerator0`
      (`PrimitiveComponent.SetCollisionResponseToAllChannels` _sphere "ECR_Block"))
    (:`NewEnumerator1`
      (`PrimitiveComponent.SetCollisionResponseToAllChannels` _sphere "ECR_Ignore")))
  (return))

(fn `Set Material`
  (params (Character :type "/Game/Blueprints/SwitchCharacter/E_Character Enum" :default "NewEnumerator0"))
  (bind _sphere (`self.Sphere`))
  (switch `/Game/Blueprints/SwitchCharacter/E_Character` Character
    (:`NewEnumerator0`
      (`PrimitiveComponent.SetMaterial` _sphere 0 "/Engine/VREditor/UI/ArrowMaterial.ArrowMaterial"))
    (:`NewEnumerator1`
      (`PrimitiveComponent.SetMaterial` _sphere 0 "/Engine/VREditor/UI/DiscMaterial.DiscMaterial")))
  (return))

(fn `UserConstructionScript`)