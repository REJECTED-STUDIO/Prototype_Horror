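; BP_SpheraTest is a test sphere that changes its physical presence and look depending on which character, Lucia or Nyxa, is switched to.
; The CharacterSwitch event calls SetCollision and SetMaterial with the character enum.
; For Lucia the sphere blocks all channels, can be stepped on and uses the arrow material; for Nyxa it ignores collision, cannot be stepped on and uses the disc material.
; Each material change also prints a debug string.
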(event `/Game/Blueprints/SwitchCharacter/BPI_SwitchCharacter.CharacterSwitch`
  (params (Characters :type "/Game/Blueprints/SwitchCharacter/E_Character Enum" :default "NewEnumerator0"))
  (`self.Set Collision` Characters)
  (`self.Set Material` Characters))

(fn `Set Collision`
  (params (NewParam :type "/Game/Blueprints/SwitchCharacter/E_Character Enum" :default "NewEnumerator0"))
  (bind _sphere (`self.Sphere`))
  (switch `/Game/Blueprints/SwitchCharacter/E_Character` NewParam
    (:`NewEnumerator0`
      (`PrimitiveComponent.SetCollisionResponseToAllChannels` _sphere "ECR_Block")
      (set `PrimitiveComponent.CanCharacterStepUpOn` "ECB_Yes" _sphere))
    (:`NewEnumerator1`
      (`PrimitiveComponent.SetCollisionResponseToAllChannels` _sphere "ECR_Ignore")
      (set `PrimitiveComponent.CanCharacterStepUpOn` "ECB_No" _sphere)))
  (return))

(fn `Set Material`
  (params (Character :type "/Game/Blueprints/SwitchCharacter/E_Character Enum" :default "NewEnumerator0"))
  (bind _sphere (`self.Sphere`))
  (switch `/Game/Blueprints/SwitchCharacter/E_Character` Character
    (:`NewEnumerator0`
      (`PrimitiveComponent.SetMaterial` _sphere 0 "/Engine/VREditor/UI/ArrowMaterial.ArrowMaterial")
      (`KismetSystemLibrary.PrintString` "Luccccia2" true true (struct :`R` 0.042671 :`B` 1.0 :`A` 1.0)))
    (:`NewEnumerator1`
      (`PrimitiveComponent.SetMaterial` _sphere 0 "/Engine/VREditor/UI/DiscMaterial.DiscMaterial")
      (`KismetSystemLibrary.PrintString` "Nyxaaaa1" true true (struct :`R` 1.0 :`B` 0.262079 :`A` 1.0))))
  (return))

(fn `UserConstructionScript`)