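; BP_ComponentEffectSwap provides helper functions that change a component's collision, material or mesh depending on the character, Lucia or Nyxa.
; Each function switches on the character value and applies that character's supplied setting to the target component.
; The three functions are independent: one sets the collision response on all channels, one replaces only the first material slot, and one swaps the static mesh.
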(fn `Set Mesh Based On Character`
  (params (Character :type "/Game/Blueprints/SwitchCharacter/E_Character Enum" :default "NewEnumerator0") (`Target Component` :type "StaticMeshComponent Object Reference") (MeshLucia :type "StaticMesh Object Reference") (MeshNyxa :type "StaticMesh Object Reference"))
  (switch `/Game/Blueprints/SwitchCharacter/E_Character` Character
    (:`NewEnumerator0`
      (`StaticMeshComponent.SetStaticMesh` `Target Component` MeshLucia))
    (:`NewEnumerator1`
      (`StaticMeshComponent.SetStaticMesh` `Target Component` MeshNyxa))))

(fn `SetCollisionBasedOnCharacter`
  (params (Character :type "/Game/Blueprints/SwitchCharacter/E_Character Enum" :default "NewEnumerator0") (`Target Component` :type "PrimitiveComponent Object Reference") (LuciaCollision :type "ECollisionResponse Enum" :default "ECR_Ignore") (NyxaParam :type "ECollisionResponse Enum" :default "ECR_Ignore"))
  (switch `/Game/Blueprints/SwitchCharacter/E_Character` Character
    (:`NewEnumerator0`
      (`PrimitiveComponent.SetCollisionResponseToAllChannels` `Target Component` LuciaCollision))
    (:`NewEnumerator1`
      (`PrimitiveComponent.SetCollisionResponseToAllChannels` `Target Component` NyxaParam))))

(fn `SetMaterialBasedOnCharacter`
  (params (Character :type "/Game/Blueprints/SwitchCharacter/E_Character Enum" :default "NewEnumerator0") (`Target Component` :type "PrimitiveComponent Object Reference") (MaterialLucia :type "Material Object Reference") (MaterialNyxa :type "Material Object Reference"))
  (switch `/Game/Blueprints/SwitchCharacter/E_Character` Character
    (:`NewEnumerator0`
      (`PrimitiveComponent.SetMaterial` `Target Component` 0 MaterialLucia))
    (:`NewEnumerator1`
      (`PrimitiveComponent.SetMaterial` `Target Component` 0 MaterialNyxa))))