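; Test actor whose Sphere component changes collision, material and mesh depending on whether the character is Lucia or Nyxa.
; The CharacterSwitch event passes the incoming character and per-character assets to BPComponentEffectSwap, which applies all three swaps.
; The construction script makes the same calls from the Character variable, but omits the collision settings and has an empty switch on Character.
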(event `/Game/Blueprints/SwitchCharacter/BPI_SwitchCharacter.CharacterSwitch`
  (params (Characters :type "/Game/Blueprints/SwitchCharacter/E_Character Enum" :default "NewEnumerator0"))
  (bind _sphere (`self.Sphere`))
  (bind _bp_componenteffectswap (`self.BP_ComponentEffectSwap`))
  (`/Game/Blueprints/BP_ComponentEffectSwap.SetCollisionBasedOnCharacter` _bp_componenteffectswap Characters _sphere (`self.LuciaCollision`) (`self.Nyxa Collision`))
  (`/Game/Blueprints/BP_ComponentEffectSwap.SetMaterialBasedOnCharacter` _bp_componenteffectswap Characters _sphere (`self.Material Lucia`) (`self.Material Nyxa`))
  (`/Game/Blueprints/BP_ComponentEffectSwap.Set Mesh Based On Character` _bp_componenteffectswap Characters _sphere (`self.Mesh Lucia`) (`self.Mesh Nyxa`)))

(fn `UserConstructionScript`
  (bind _character (`self.Character`))
  (bind _sphere (`self.Sphere`))
  (bind _bp_componenteffectswap (`self.BP_ComponentEffectSwap`))
  (switch `/Game/Blueprints/SwitchCharacter/E_Character` _character
    (:`NewEnumerator0`
      _)
    (:`NewEnumerator1`
      _))
  (`/Game/Blueprints/BP_ComponentEffectSwap.SetCollisionBasedOnCharacter` _bp_componenteffectswap _character _sphere "ECR_Ignore" "ECR_Ignore")
  (`/Game/Blueprints/BP_ComponentEffectSwap.SetMaterialBasedOnCharacter` _bp_componenteffectswap _character _sphere (`self.Material Lucia`) (`self.Material Nyxa`))
  (`/Game/Blueprints/BP_ComponentEffectSwap.Set Mesh Based On Character` _bp_componenteffectswap _character _sphere (`self.Mesh Lucia`) (`self.Mesh Nyxa`)))