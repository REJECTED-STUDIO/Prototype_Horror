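; BP_WorldSwitch adjusts the level's sun lighting when the active character changes between Lucia and Nyxa.
; Its CharacterSwitch event passes the character to the Light function, which finds the level's Directional Lights and changes only the first one returned.
; Lucia sets that light's intensity to the day value and Nyxa to the night value, as an immediate change with no blend.
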(event `/Game/Blueprints/SwitchCharacter/BPI_SwitchCharacter.CharacterSwitch`
  (params (Characters :type "/Game/Blueprints/SwitchCharacter/E_Character Enum" :default "NewEnumerator0"))
  (`self.Light` Characters))

(fn `Light`
  (params (Character :type "/Game/Blueprints/SwitchCharacter/E_Character Enum" :default "NewEnumerator0"))
  (bind _outactors (`GameplayStatics.GetAllActorsOfClass` "/Script/Engine.DirectionalLight"))
  (switch `/Game/Blueprints/SwitchCharacter/E_Character` Character
    (:`NewEnumerator0`
      (bind _lightcomponent (`Light.LightComponent` (`|GetArrayItem` _outactors)))
      (`LightComponent.SetIntensity` _lightcomponent (`self.Sun DAY Intensity`)))
    (:`NewEnumerator1`
      (`LightComponent.SetIntensity` _lightcomponent (`self.Sun Night Intensity`))))
  (return))

(fn `UserConstructionScript`)