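; Camera trigger volume that blends the player's view to its assigned fixed camera, active only for Nyxa; switching to Lucia makes the box ignore collision.
; Entering activates the camera, or queues it as the character's next camera if one is already active, to handle overlapping triggers.
; Exiting clears its own queued entry, hands off to another queued camera, or blends back to the character and restores its saved control rotation.
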(event `/Game/Blueprints/SwitchCharacter/BPI_SwitchCharacter.CharacterSwitch`
  (params (Characters :type "/Game/Blueprints/SwitchCharacter/E_Character Enum" :default "NewEnumerator0"))
  (bind _box (`self.Box`))
  ;[1 1 1] Nyxa Can use Fixed Cam
  (switch `/Game/Blueprints/SwitchCharacter/E_Character` Characters
    (:`NewEnumerator0`
      (`PrimitiveComponent.SetCollisionResponseToAllChannels` _box "ECR_Ignore"))
    (:`NewEnumerator1`
      (`PrimitiveComponent.SetCollisionResponseToAllChannels` _box "ECR_Overlap"))))

(event `self.Box.OnComponentBeginOverlap`
  (params (OverlappedComponent :type "PrimitiveComponent Object Reference") (OtherActor :type "Actor Object Reference") (OtherComp :type "PrimitiveComponent Object Reference") (OtherBodyIndex :type Integer) (bFromSweep :type Boolean) (SweepResult :type "HitResult Structure (by ref)"))
  (bind _player_ref (`self.Player Ref`))
  ;[1 1 1] Overlap Camera
  (bind _asbp_third_person_character (cast `/Game/ThirdPerson/Blueprints/BP_ThirdPersonCharacter` OtherActor))
  (set `self.Player Ref` _asbp_third_person_character)
  ;;[0 0 0] Set Camera Ref
  (`/Engine/EditorBlueprintResources/StandardMacros.IsValid` (`/Game/ThirdPerson/Blueprints/BP_ThirdPersonCharacter.NextFixedCam` _player_ref)
    (:`Is Valid`
      (set `/Game/ThirdPerson/Blueprints/BP_ThirdPersonCharacter.NextFixedCam` (`self.BP_Camera`) (`self.Player Ref`)))
    (:`Is Not Valid`
      (`/Engine/EditorBlueprintResources/StandardMacros.IsValid` (`/Game/ThirdPerson/Blueprints/BP_ThirdPersonCharacter.FixedCameraRef` _player_ref)
        (:`Is Valid`
          (set `/Game/ThirdPerson/Blueprints/BP_ThirdPersonCharacter.NextFixedCam` (`self.BP_Camera`) (`self.Player Ref`)))
        (:`Is Not Valid`
          (set `/Game/ThirdPerson/Blueprints/BP_ThirdPersonCharacter.FixedCameraRef` (`self.BP_Camera`) _player_ref)
          (set `/Game/Blueprints/Camera/BP_FixedCamera.FixedCameraUse` true (`self.BP_Camera`))
          (`PlayerController.SetViewTargetWithBlend` (`GameplayStatics.GetPlayerController` 0) (`self.BP_Camera`) (`self.Blend Time`) (`self.Blend Func`) 0.0 false)
          (set `Pawn.bUseControllerRotationYaw` false _player_ref))))))

(event `self.Box.OnComponentEndOverlap`
  (params (OverlappedComponent :type "PrimitiveComponent Object Reference") (OtherActor :type "Actor Object Reference") (OtherComp :type "PrimitiveComponent Object Reference") (OtherBodyIndex :type Integer))
  (bind _player_ref (`self.Player Ref`))
  (bind _nextfixedcam (`/Game/ThirdPerson/Blueprints/BP_ThirdPersonCharacter.NextFixedCam` _player_ref))
  ;[1 1 1] Next Camera Or End Overlap Cam
  (bind _asbp_third_person_character (cast `/Game/ThirdPerson/Blueprints/BP_ThirdPersonCharacter` OtherActor))
  ;;[0 0 0] Next Camera or End
  (if (== (`/Game/ThirdPerson/Blueprints/BP_ThirdPersonCharacter.NextFixedCam` (`self.Player Ref`)) (`self.BP_Camera`))
    (set `/Game/ThirdPerson/Blueprints/BP_ThirdPersonCharacter.NextFixedCam` null (`self.Player Ref`))
    (else
      (`/Engine/EditorBlueprintResources/StandardMacros.IsValid` _nextfixedcam
        (:`Is Valid`
          (bind _output_get (set `/Game/ThirdPerson/Blueprints/BP_ThirdPersonCharacter.FixedCameraRef` _nextfixedcam _player_ref))
          (set `/Game/ThirdPerson/Blueprints/BP_ThirdPersonCharacter.NextFixedCam` null (`self.Player Ref`))
          (set `/Game/Blueprints/Camera/BP_FixedCamera.FixedCameraUse` true _output_get)
          (`PlayerController.SetViewTargetWithBlend` (`GameplayStatics.GetPlayerController` 0) _output_get (`self.Blend Time`) (`self.Blend Func`) 0.0 false)
          (set `Pawn.bUseControllerRotationYaw` false _player_ref))
        (:`Is Not Valid`
          (set `/Game/ThirdPerson/Blueprints/BP_ThirdPersonCharacter.FixedCameraRef` null _player_ref)
          (set `/Game/Blueprints/Camera/BP_FixedCamera.FixedCameraUse` false (`self.BP_Camera`))
          (`PlayerController.SetViewTargetWithBlend` (`GameplayStatics.GetPlayerController` 0) _asbp_third_person_character (`self.Blend Time`) (`self.Blend Func`) 0.0 false)
          (`Controller.SetControlRotation` (`GameplayStatics.GetPlayerController` 0) (`/Game/ThirdPerson/Blueprints/BP_ThirdPersonCharacter.Old Control Rottation` _asbp_third_person_character)))))))

(fn `UserConstructionScript`
  (`BoxComponent.SetBoxExtent` (`self.Box`) (`self.BoxSize`) true))