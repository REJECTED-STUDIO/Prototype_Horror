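; BP_ManipulationWorld is an actor that changes the look of the world when the active character switches between Lucia and Nyxa.
; Its CharacterSwitch event passes the character to two functions, Light and TestMaterial.
; Light finds the first DirectionalLight in the level and sets its intensity, brighter for Lucia and dimmer for Nyxa.
; TestMaterial swaps the Sphere's material per character and prints a debug string.
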(event `/Game/Mechanic/SwitchCharacter/BPI_SwitchCharacter.CharacterSwitch`
  (params (Characters :type "/Game/Mechanic/SwitchCharacter/E_Character Enum" :default "NewEnumerator0"))
  (`self.Light` Characters)
  (`self.TestMaterial` Characters))

(fn `Light`
  (params (Character :type "/Game/Mechanic/SwitchCharacter/E_Character Enum" :default "NewEnumerator0"))
  (bind _outactors (`GameplayStatics.GetAllActorsOfClass` "/Script/Engine.DirectionalLight"))
  (switch `/Game/Mechanic/SwitchCharacter/E_Character` Character
    (:`NewEnumerator0`
      (bind _lightcomponent (`Light.LightComponent` (`|GetArrayItem` _outactors)))
      (`LightComponent.SetIntensity` _lightcomponent 3.0))
    (:`NewEnumerator1`
      (`LightComponent.SetIntensity` _lightcomponent 0.5)))
  (return))

(fn `TestMaterial`
  (params (Character :type "/Game/Mechanic/SwitchCharacter/E_Character Enum" :default "NewEnumerator0"))
  (switch `/Game/Mechanic/SwitchCharacter/E_Character` Character
    (:`NewEnumerator0`
      (`PrimitiveComponent.SetMaterial` (`self.Sphere`) 0 "/Engine/VREditor/UI/ArrowMaterial.ArrowMaterial")
      (`KismetSystemLibrary.PrintString` "Luccccia2" true true (struct :`R` 0.042671 :`B` 1.0 :`A` 1.0)))
    (:`NewEnumerator1`
      (`PrimitiveComponent.SetMaterial` (`self.Sphere`) 0 "/Engine/VREditor/UI/DiscMaterial.DiscMaterial")
      (`KismetSystemLibrary.PrintString` "Nyxaaaa1" true true (struct :`R` 1.0 :`B` 0.262079 :`A` 1.0))))
  (return))

(fn `UserConstructionScript`)